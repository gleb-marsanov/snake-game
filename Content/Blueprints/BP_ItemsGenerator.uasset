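; BP_ItemsGenerator spawns food, speed-up and teleport pickups at random XY positions within a square area at a fixed height.
; On BeginPlay it spawns one food and starts looping timers that add speed-ups frequently and teleports less often.
; Each food binds its OnDestroyed event to spawn a replacement, keeping one food from this generator in play.
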(event `self.ReceiveBeginPlay`
  (`self.SpawnFood`)
  (`KismetSystemLibrary.K2_SetTimerDelegate` (delegate `SpawnSpeedUp`) 5.0 true)
  (`KismetSystemLibrary.K2_SetTimerDelegate` (delegate `SpawnTeleport`) 30.0 true))

(event `SpawnTeleport`
  (`|SpawnActorFromClass` "/Game/Blueprints/BP_Teleport.BP_Teleport_C" (`KismetMathLibrary.MakeTransform` (`KismetMathLibrary.MakeVector` (`KismetMathLibrary.RandomFloatInRange` -800.0 800.0) (`KismetMathLibrary.RandomFloatInRange` -800.0 800.0) -100.0)) "Undefined" "MultiplyWithRoot" null null))

(event `SpawnSpeedUp`
  (`|SpawnActorFromClass` "/Game/Blueprints/BP_SpeedUp.BP_SpeedUp_C" (`KismetMathLibrary.MakeTransform` (`KismetMathLibrary.MakeVector` (`KismetMathLibrary.RandomFloatInRange` -800.0 800.0) (`KismetMathLibrary.RandomFloatInRange` -800.0 800.0) -100.0)) "Undefined" "MultiplyWithRoot" null null))

(event `SpawnFood`
  (bind _returnvalue (`|SpawnActorFromClass` "/Game/Blueprints/BP_Food.BP_Food_C" (`KismetMathLibrary.MakeTransform` (`KismetMathLibrary.MakeVector` (`KismetMathLibrary.RandomFloatInRange` -800.0 800.0) (`KismetMathLibrary.RandomFloatInRange` -800.0 800.0) -100.0)) "Undefined" "MultiplyWithRoot" null null))
  (add `self.OnDestroyed` _returnvalue (delegate `FoodDestroyed`)))

(event `FoodDestroyed` :!signature `self.OnDestroyed`
  (params (DestroyedActor :type "Actor Object Reference"))
  (`self.SpawnFood`))

(fn `UserConstructionScript`)