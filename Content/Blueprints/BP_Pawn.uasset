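; BP_Pawn is a player pawn that manages input mode and shows the game over screen when it is destroyed.
; On BeginPlay it binds to its own OnDestroyed event, switches to game-only input and hides the mouse cursor.
; The destroy handler creates and displays WBP_GameOver, switches to UI-only input focused on that widget and shows the cursor.
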(event `self.ReceiveBeginPlay`
  (bind _returnvalue (`GameplayStatics.GetPlayerController` 0))
  (add `Actor.OnDestroyed` (delegate `OnDestroy_Event`))
  (`WidgetBlueprintLibrary.SetInputMode_GameOnly` _returnvalue)
  (set `PlayerController.bShowMouseCursor` false _returnvalue))

(event `OnDestroy_Event`
  (params (DestroyedActor :type "Actor Object Reference"))
  (bind _returnvalue (`GameplayStatics.GetPlayerController` 0))
  (bind _returnvalue_2 (`|CreateWidget` "/Game/Blueprints/WBP_GameOver.WBP_GameOver_C" (`GameplayStatics.GetPlayerController` 0)))
  (`UserWidget.AddToViewport` _returnvalue_2 0)
  (`WidgetBlueprintLibrary.SetInputMode_UIOnlyEx` _returnvalue _returnvalue_2)
  (set `PlayerController.bShowMouseCursor` true _returnvalue))

(fn `UserConstructionScript`)